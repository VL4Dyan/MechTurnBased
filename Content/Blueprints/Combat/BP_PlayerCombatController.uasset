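; Player controller for grid-based combat that handles tile hover, tile selection and action signals from the combat UI.
; On BeginPlay it gets the grid manager from the combat game mode, spawns cursor and selection highlights, and creates the combat UI.
; Each tick a cursor trace converts to grid indexes to move the hover highlight; clicks select tiles outside action state.
; UI signals resolve into decisions, shown as green tile highlights during action state.
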(event `self.ReceiveBeginPlay`
  (bind _returnvalue (`KismetMathLibrary.MakeTransform` (0.0 0.0 500.0)))
  (bind _asbp_combat_mode (cast `/Game/Blueprints/Combat/BP_CombatMode` (`GameplayStatics.GetGameMode`)))
  (bind _returnvalue_2 (`CombatMode.GetCombatGridManagerRef` _asbp_combat_mode))
  (set `self.CombatGridManagerRef` _returnvalue_2)
  (bind _returnvalue_3 (`|SpawnActorFromClass` "/Game/Blueprints/Combat/Grid/BP_TileHighlight.BP_TileHighlight_C" _returnvalue "Undefined" "OverrideRootScale" null null))
  (set `self.BP_CursorTileHighlight` _returnvalue_3)
  (bind _returnvalue_4 (`|SpawnActorFromClass` "/Game/Blueprints/Combat/Grid/BP_TileHighlight.BP_TileHighlight_C" _returnvalue "Undefined" "OverrideRootScale" null null))
  (set `self.BP_SelectedTileHighlight` _returnvalue_4)
  (`self.SetDefaultHighlightColors`)
  (bind _returnvalue_5 (`|CreateWidget` "/Game/Blueprints/Combat/BP_CombatUI.BP_CombatUI_C"))
  (`UserWidget.AddToViewport` _returnvalue_5 0)
  (set `/Game/Blueprints/Combat/BP_CombatUI.ControllerRef` self _returnvalue_5))

(event `self.ReceiveTick`
  (params (DeltaSeconds :type "Float (single-precision)"))
  (bind _matrixindexes (`self.ConvertCursorHitToIndexes`))
  (bind (_tileout _returnvalue) (`self.TryGetTempSelectedTile` _matrixindexes))
  (if _returnvalue
    (`self.K2_SetActorLocation` (`self.BP_CursorTileHighlight`) (`.AbsoluteCoordinates` (break `TileData` _tileout)) false false)
    (else
      (`self.K2_SetActorLocation` (`self.BP_CursorTileHighlight`) (0.0 0.0 500.0) false false))))

(event `InputAction|LeftMouseClick`
  (params (Key :type "Key Structure"))
  (:`Pressed`
    (if (`self.bActionState`)
      (`self.ConvertCursorHitToIndexes`)
      (else
        (`self.SelectTile`)))))

(fn `ConvertCursorHitToIndexes`
  (returns (MatrixIndexes :type "MatrixIndexes Structure"))
  (bind _returnvalue (`CombatGridManager.ConvertCoordinatesToIndexes` (`self.CombatGridManagerRef`) (`.Location` (`GameplayStatics.BreakHitResult` (`self.GetHitResultUnderCursorForObjects` (`GameplayStatics.GetPlayerController` 0) (`|MakeArray` "ObjectTypeQuery7" :!type "EObjectTypeQuery Enum") true)))))
  (return _returnvalue))

(fn `ProcessUISignal`
  (params (Signal :type Integer))
  (bind _returnvalue (`self.GetActionResultBasedOnUISignal` Signal))
  (set `self.CurrentDecisions` _returnvalue)
  (if (`self.bActionState`)
    (for _array_element (`self.CurrentDecisions`)
      (bind _tileout (`self.TryGetTempSelectedTile` (`TileTargetingResult.TileIndex` _array_element)))
      (bind _returnvalue_2 (`|SpawnActorFromClass` "/Game/Blueprints/Combat/Grid/BP_TileHighlight.BP_TileHighlight_C" (`KismetMathLibrary.Conv_VectorToTransform` (`.AbsoluteCoordinates` (break `TileData` _tileout))) "Undefined" "OverrideRootScale" null null))
      (`/Game/Blueprints/Combat/Grid/BP_TileHighlight.SetTileHighlightMaterialColor` _returnvalue_2 (struct :`G` 0.791667 :`B` 0.020146 :`A` 1.0))
      (`KismetArrayLibrary.Array_Add` (`self.TempTileHighlights`) _returnvalue_2))))

(fn `SelectTile`
  (locals (ResultIndexes :type "MatrixIndexes Structure") (ResultTileDatas :type " Structure") (SelectionSuccess :type Boolean) (ResultTileData :type "TileData Structure"))
  (bind _matrixindexes (`self.ConvertCursorHitToIndexes`))
  (`self.SetSelectedTile` _matrixindexes))

(fn `SetDefaultHighlightColors`
  (`/Game/Blueprints/Combat/Grid/BP_TileHighlight.SetTileHighlightMaterialColor` (`self.BP_CursorTileHighlight`) (struct :`R` 1.0 :`G` 0.383678 :`B` 0.244792 :`A` 1.0))
  (`/Game/Blueprints/Combat/Grid/BP_TileHighlight.SetTileHighlightMaterialColor` (`self.BP_SelectedTileHighlight`) (struct :`R` 1.0 :`G` 0.184314 :`A` 1.0)))

(fn `UserConstructionScript`)