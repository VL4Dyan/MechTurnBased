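; BP_CombatCamera is a player-controlled camera pawn for combat, with panning, rotation and zoom.
; Forward and Right axes move it along yaw-based directions with pitch zeroed, so tilt does not affect movement.
; Holding the middle mouse button enables yaw and pitch rotation of the whole actor.
; Zoom inputs reposition the PlayerVision component through CalculateZoomTransform, with step and distance limits set in the construction script.
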(event `self.ReceiveBeginPlay`
  (`self.SetDefaultPosition` (`self.PlayerVision`)))

(event `InputAxis|Forward`
  (params (AxisValue :type "Float (single-precision)"))
  (bind (_returnvalue_roll _returnvalue_pitch _returnvalue_yaw) (`KismetMathLibrary.BreakRotator` (`self.K2_GetActorRotation`)))
  ;[1 1 1] Movement
  (`self.AddMovementInput` (`KismetMathLibrary.GetForwardVector` (`KismetMathLibrary.MakeRotator` _returnvalue_roll 0.0 _returnvalue_yaw)) AxisValue))

(event `InputAxis|Right`
  (params (AxisValue :type "Float (single-precision)"))
  (bind (_returnvalue_roll _returnvalue_pitch _returnvalue_yaw) (`KismetMathLibrary.BreakRotator` (`self.K2_GetActorRotation`)))
  ;[1 1 1] Movement
  (`self.AddMovementInput` (`KismetMathLibrary.GetRightVector` (`KismetMathLibrary.MakeRotator` _returnvalue_roll 0.0 _returnvalue_yaw)) AxisValue))

(event `InputAction|ZoomIn`
  (params (Key :type "Key Structure"))
  (:`Pressed`
    (bind _returnvalue (`self.CalculateZoomTransform` (`SceneComponent.GetRelativeTransform` (`self.PlayerVision`)) -1.0))
    (`SceneComponent.K2_SetRelativeTransform` (`self.PlayerVision`) _returnvalue false false)))

(event `InputAction|ZoomOut`
  (params (Key :type "Key Structure"))
  (:`Pressed`
    (bind _returnvalue (`self.CalculateZoomTransform` (`SceneComponent.GetRelativeTransform` (`self.PlayerVision`)) 1.0))
    (`SceneComponent.K2_SetRelativeTransform` (`self.PlayerVision`) _returnvalue false false)))

(event `Key|MiddleMouseButton`
  (params (Key :type "Key Structure"))
  (:`Pressed`
    (set `self.CameraRotationEnabled` true))
  (:`Released`
    (set `self.CameraRotationEnabled` false)))

(event `InputAxis|LookHorizontally`
  (params (AxisValue :type "Float (single-precision)"))
  (if (`self.CameraRotationEnabled`)
    (`self.K2_AddActorWorldRotation` (`KismetMathLibrary.MakeRotator` 0.0 0.0 (* AxisValue (`self.CameraRotationSpeed`))))))

(event `InputAxis|LookVertically`
  (params (AxisValue :type "Float (single-precision)"))
  (if (`self.CameraRotationEnabled`)
    (`self.K2_AddActorWorldRotation` (`KismetMathLibrary.MakeRotator` 0.0 (* AxisValue (`self.CameraRotationSpeed`))))))

(fn `UserConstructionScript`
  (set `self.MaxZoomDistance` 1200.0)
  (set `self.MinZoomDistance` 500.0)
  (set `self.ZoomStep` 50.0))