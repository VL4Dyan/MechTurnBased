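; BP_OneTileUnit is a combat unit, apparently single-tile, that moves along a path of world points.
; Its Moveto event spawns a BP_SplinePathway at the first point and sets its spline points to the supplied locations.
; A timeline drives the unit's location and rotation by distance along that spline, with play rate divided by segment count so travel time scales with path length.
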(event `self.ReceiveBeginPlay`)

(event `/Game/Blueprints/Combat/Units/BP_ActiveCombatObject.MoveTo`
  (params (`New Location` :type "Array of Vector Structure (by ref)"))
  (bind _timeline_0 (`self.Timeline_0`))
  (bind _returnvalue (- (`KismetArrayLibrary.Array_Length` `New Location`) 1))
  (bind _returnvalue_2 (`KismetMathLibrary.Lerp` 0.0 (`SplineComponent.GetSplineLength` (`/Game/Blueprints/Combat/Units/BP_SplinePathway.Spline` (`self.Pathway`))) (`self.Alpha`)))
  (bind _returnvalue_3 (`|SpawnActorFromClass` "/Game/Blueprints/Combat/Units/BP_SplinePathway.BP_SplinePathway_C" (`KismetMathLibrary.MakeTransform` (`|GetArrayItem` `New Location`)) "AlwaysSpawn" "OverrideRootScale" null null))
  (bind _output_get (set `self.Pathway` _returnvalue_3))
  (`SplineComponent.SetSplinePoints` (`/Game/Blueprints/Combat/Units/BP_SplinePathway.Spline` _output_get) `New Location` "World" true)
  (if (> _returnvalue 0)
    (bind _output_get_2 (set `self.PlayRate` (/ 2.0 (`KismetMathLibrary.Conv_IntToDouble` _returnvalue))))
    (`TimelineComponent.SetPlayRate` _timeline_0 _output_get_2)
    (bind (_direction _newtrack_0) (`Timeline|Timeline_0` :!via `PlayFromStart` :!label _label)
      (:`Update`
        (set `self.Alpha` _newtrack_0)
        (`self.K2_SetActorLocationAndRotation` (`SplineComponent.GetLocationAtDistanceAlongSpline` (`/Game/Blueprints/Combat/Units/BP_SplinePathway.Spline` (`self.Pathway`)) _returnvalue_2 "World") (`SplineComponent.GetRotationAtDistanceAlongSpline` (`/Game/Blueprints/Combat/Units/BP_SplinePathway.Spline` (`self.Pathway`)) _returnvalue_2 "World"))))
    (else
      (bind _output_get_3 (set `self.PlayRate` 1.0))
      (`TimelineComponent.SetPlayRate` _timeline_0 _output_get_3)
      (goto _label :!via `PlayFromStart`))))

(fn `UserConstructionScript`)