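; Mech movement component for grid-based combat that produces and processes movement action results.
; On BeginPlay it creates a MovementLogic object linked to the combat mode's grid manager.
; GetActionResult builds an ActionResult and has MovementLogic fill its targets from the component's position using a fixed distance; its return node is unwired.
; ProcessActionResultUpdates writes replacement data for updated and related tiles, currently copying current tile data without changing any fields.
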(event `self.ReceiveBeginPlay`
  (bind _returnvalue (`|GenericCreateObject` "/Script/MechTurnBased.MovementLogic" self))
  (bind _output_get (set `self.MovementLogic` _returnvalue))
  (bind _ascombat_mode (cast `CombatMode` (`GameplayStatics.GetGameMode`)))
  (set `MovementLogic.CombatGridManagerRef` (`CombatMode.CombatGridManager` _ascombat_mode) _output_get)
  (set `self.ComponentType` "CompType_Movement"))

(fn `GetActionResult`
  (returns (ReturnValue :type "ActionResult Object Reference"))
  (locals (ActionResult :type "ActionResult Object Reference"))
  (bind _returnvalue (`|GenericCreateObject` "/Script/MechTurnBased.ActionResult" self))
  (bind _output_get (set `local.ActionResult` _returnvalue))
  (`ActionResult.Initialize` _output_get self)
  (`MovementLogic.SetTargetsInActionResultViaMovementLogicProcessing` (`self.MovementLogic`) (`local.ActionResult`) (`self.ComponentFunctionalityPosition`) 3))

(fn `ProcessActionResultUpdates`
  (params (ActionResult :type "ActionResult Object Reference"))
  (bind _outtiledataupdates (`ActionResult.GetUpdatesToProcess` ActionResult))
  (for _array_element _outtiledataupdates
    (bind (_outtileindex _outtiledata) (`TileDataUpdate.GetCurrentTileInfo` _array_element))
    (bind _structout (setmembers `TileData` :`StructRef` _outtiledata :`TileHolder` null))
    (`TileDataUpdate.SetTileDataReplacement` _array_element _structout)
    (bind _returnvalue (`TileDataUpdate.GetRelatedTileDataUpdates` _array_element))
    (for _array_element_2 _returnvalue
      (bind (_outtileindex_2 _outtiledata_2) (`TileDataUpdate.GetCurrentTileInfo` _array_element_2))
      (bind _structout_2 (setmembers `TileData` :`StructRef` _outtiledata_2 :`TileHolder` null))
      (`TileDataUpdate.SetTileDataReplacement` _array_element_2 _structout_2))))