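; BP_LinearWeapon is a mech attack component that damages grid object components along a line of fire.
; At BeginPlay it builds a TargetingLogic object wired to the combat mode's grid manager and a trace channel.
; GetActionResult line-traces a short range from the component to fill a new ActionResult, then queues a one-point hull reduction for each targeted component state.
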(event `self.ReceiveBeginPlay`
  (bind _returnvalue (`|GenericCreateObject` "/Script/MechTurnBased.TargetingLogic" self))
  (bind _output_get (set `self.TargetingLogic` _returnvalue))
  (bind _ascombat_mode (cast `CombatMode` (`GameplayStatics.GetGameMode`)))
  (bind _returnvalue_2 (`CombatMode.GetCombatGridManagerRef` _ascombat_mode))
  (set `TargetingLogic.CombatGridManagerRef` _returnvalue_2 _output_get)
  (set `TargetingLogic.CollisionChannel` "ECC_GameTraceChannel2" _output_get)
  (set `self.ComponentType` "CompType_Attack"))

(fn `GetActionResult`
  (returns (ReturnValue :type "ActionResult Object Reference"))
  (locals (ActionResult :type "ActionResult Object Reference"))
  (bind _returnvalue (`|GenericCreateObject` "/Script/MechTurnBased.ActionResult" self))
  (bind _output_get (set `local.ActionResult` _returnvalue))
  (`ActionResult.Initialize` _output_get self)
  (`TargetingLogic.SetTargetsInActionResultViaLineTrace` (`self.TargetingLogic`) (`local.ActionResult`) (`self.ComponentFunctionalityPosition`) 3)
  (`self.ProcessActionResultUpdates` (`local.ActionResult`))
  (return (`local.ActionResult`)))

(fn `ProcessActionResultUpdates`
  (params (ActionResultToProcess :type "ActionResult Object Reference"))
  (locals (GridObjCompState :type "GridObjectComponentState Structure"))
  (bind (_outtiledataupdates _outgridobjcompstateupdates) (`ActionResult.GetUpdatesToProcess` ActionResultToProcess))
  (for _array_element _outgridobjcompstateupdates
    (bind _outgridobjcompstate (`GridObjectComponentStateUpdate.GetCurrentComponentState` _array_element))
    (`GridObjectComponentStateUpdate.SetGridObjectComponentStateReplacement` _array_element (make `GridObjectComponentState` (- (break `GridObjectComponentState` _outgridobjcompstate) 1)))))