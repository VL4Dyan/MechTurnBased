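; BP_CombatMode sets up a grid-based combat encounter when play begins.
; It spawns a temporary BP_TileChecker, passes it to ScanGrid, then destroys it.
; SetDefaultCombatPlayerUnits then spawns several default one-tile units for each entry in SpawnPoints and hands each to PlaceCombatUnitOnGrid with that spawn point.
; ScanGrid and PlaceCombatUnitOnGrid are defined outside this graph.
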(event `self.ReceiveBeginPlay`
  (bind _returnvalue (`|SpawnActorFromClass` "/Game/Blueprints/Combat/Grid/BP_TileChecker.BP_TileChecker_C" (`KismetMathLibrary.MakeTransform` (0.0 0.0 0.0)) "Undefined" "OverrideRootScale" null null))
  (`self.ScanGrid` _returnvalue)
  (`self.K2_DestroyActor` _returnvalue)
  (`self.SetDefaultCombatPlayerUnits`))

(fn `SetDefaultCombatPlayerUnits`
  (for _array_element (`self.SpawnPoints`)
    (for _ (range 3)
      (bind _returnvalue (`|SpawnActorFromClass` "/Game/Blueprints/Combat/Units/BP_OneTileUnit.BP_OneTileUnit_C" (`KismetMathLibrary.MakeTransform` (0.0 0.0 0.0)) "Undefined" "OverrideRootScale" null null))
      (`self.PlaceCombatUnitOnGrid` _returnvalue _array_element))))

(fn `UserConstructionScript`)